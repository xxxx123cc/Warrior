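; BP_HeroCharacter is the player character Blueprint, whose only active logic toggles the pause menu from the IA_PauseMenu input action.
; When opening, it async-loads the WBP_PauseScreen class, creates the widget, adds it to the viewport and sets IsPause.
; When closing, it removes the widget, restores game-only input, unpauses and clears the flag.
; The opening branch itself neither pauses the game nor changes input mode.
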(event Input|EnhancedActionEvents|EnhancedInputActionIA_PauseMenu
  (params (ActionValue :type Boolean) (ElapsedSeconds :type Float%20%28double-precision%29) (TriggeredSeconds :type Float%20%28double-precision%29) (InputAction :type Input%20Action%20Object%20Reference :default "/Game/PlayerCharacter/Input/Actions/IA_PauseMenu.IA_PauseMenu"))
  (:Started
    (if (Variables|Default|GetisPause)
      (Widget|RemovefromParent (Variables|Default|GetPause%20Widget))
      (Class|WarriorFunctionLibrary|ToggleInputMode "GameOnly")
      (Game|SetGamePaused false)
      (Variables|Default|SetisPause false)
      (else
        (bind _class (Utilities|AsyncLoadClassAsset "/Game/Wideget/GameMode/WBP_PauseScreen.WBP_PauseScreen_C")
          (:Completed
            (bind _as用户控件 (Utilities|Casting|CastToUserWidgetClass _class))
            (bind _returnvalue (UserInterface|CreateWidget _as用户控件))
            (bind _output_get (Variables|Default|SetPause%20Widget _returnvalue))
            (UserInterface|Viewport|AddtoViewport _output_get 0)
            (Variables|Default|SetisPause true)))))))

(event EventBeginPlay)

(event Collision|EventActorBeginOverlap
  (params (OtherActor :type Actor%20Object%20Reference)))

(event EventTick
  (params (DeltaSeconds :type Float%20%28single-precision%29)))

(fn ConstructionScript)