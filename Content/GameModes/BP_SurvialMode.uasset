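; Survival game mode Blueprint that presents wave progress and match outcome to the player, reacting to survival state-change events bound on BeginPlay.
; Wave states spawn text widgets: countdown banners while waiting or after completion, plain banners for the wave number and a last-wave notice.
; The final wave also overrides the enemy spawn delay.
; Victory or player death clears widgets, fades the camera to black, then async-loads and shows the win or lose screen.
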(event Custom|游戏模式状态改变
  (params (CurrentState :type EWarriorSurvailGameModeState%20Enum :default "WaitSpawnNewWave"))
  (switch Utilities|FlowControl|Switch|SwitchonEWarriorSurvailGameModeState CurrentState
    (:WaitSpawnNewWave
      (CallFunction|创建可视化波次 "New Wave Coming in" (Variables|Default|GetSpawnNewWaveWaitTime)))
    (:SpawningNewWave
      (CallFunction|创建界面（无倒计时显示） (Utilities|Text|FormatText "Wave  {CurrentWaveCount}" (Variables|Default|GetCurrentWaveIndex)))
      (if (== (Variables|Default|GetCurrentWaveIndex) (Variables|Default|GetTotalWavesToSpawn))
        (Variables|Default|SetSpawnEnemiesDelayTime 4.0)
        (Utilities|FlowControl|Delay 2.0)
        (CallFunction|创建界面（无倒计时显示） "Last Wave")))
    (:WaveCompleted
      (CallFunction|创建可视化波次 (Utilities|Text|FormatText "Wave  {CurrentWaveCount}  Complete" (Variables|Default|GetCurrentWaveIndex)) (Variables|Default|GetWaveCompletedWaitTime)))
    (:AllWaveDone
      (Utilities|FlowControl|Delay 0.2)
      (Viewport|RemoveAllWidgets)
      (CameraFades|StartCameraFade :self (Game|GetPlayerCameraManager 0) :ToAlpha 1.0 :Duration 2.0 :bHoldWhenFinished true)
      (Utilities|FlowControl|Delay 3.0)
      (bind _class (Utilities|AsyncLoadClassAsset "/Game/Wideget/GameMode/WBP_WinScreen.WBP_WinScreen_C")
        (:Completed
          (bind _as用户控件 (Utilities|Casting|CastToUserWidgetClass _class))
          (bind _returnvalue (UserInterface|CreateWidget _as用户控件))
          (UserInterface|Viewport|AddtoViewport _returnvalue 0))))
    (:PlayerDied
      (Viewport|RemoveAllWidgets)
      (CameraFades|StartCameraFade :self (Game|GetPlayerCameraManager 0) :ToAlpha 1.0 :Duration 2.0 :bHoldWhenFinished true)
      (Utilities|FlowControl|Delay 2.0)
      (bind _class_2 (Utilities|AsyncLoadClassAsset "/Game/Wideget/GameMode/WBP_LoseScreen.WBP_LoseScreen_C")
        (:Completed
          (bind _as用户控件_2 (Utilities|Casting|CastToUserWidgetClass _class_2))
          (bind _returnvalue_2 (UserInterface|CreateWidget _as用户控件_2))
          (UserInterface|Viewport|AddtoViewport _returnvalue_2 0))))))

(event EventBeginPlay
  (EventDispatchers|BindEventtoOnSurvialGameModeStateChanged (delegate Custom|游戏模式状态改变)))

(event EventTick
  (params (DeltaSeconds :type Float%20%28single-precision%29)))

(fn ConstructionScript)

(fn 创建可视化波次
  (params (TextToDisplay :type Text) (TotalTime :type Float%20%28double-precision%29))
  (bind _returnvalue (Game|ConstructObjectfromClass "/Game/Wideget/GameMode/WBP_WaveTextWithContext.WBP_WaveTextWithContext_C"))
  (UserInterface|Viewport|AddtoViewport _returnvalue 0)
  (Rendering|Components|TextRender|SetText (Variables|/Game/Wideget/GameMode/WBP_WaveTextWithContext.WBP_WaveTextWithContext_C|GetWarriorTextBox_WaveText _returnvalue) TextToDisplay)
  (Default|开始倒计时 _returnvalue TotalTime))

(fn 创建界面（无倒计时显示）
  (params (InText :type Text))
  (bind _returnvalue (Game|ConstructObjectfromClass "/Game/Wideget/GameMode/WBP_WaveTextWithNoContext1.WBP_WaveTextWithNoContext1_C"))
  (UserInterface|Viewport|AddtoViewport _returnvalue 0)
  (Rendering|Components|TextRender|SetText (Variables|/Game/Wideget/GameMode/WBP_WaveTextWithNoContext1.WBP_WaveTextWithNoContext1_C|GetWarriorTextBox_WaveText _returnvalue) InText))