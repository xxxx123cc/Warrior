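; Base projectile Blueprint, filed under EnemyCharacter, that handles a projectile's cosmetic audio and Niagara effects.
; BeginPlay plays the spawn sound, attaches a flight sound that stops with the projectile, and spawns a launch effect aligned to its forward vector.
; OnSpawnProjectileHitFx plays the hit sound and effect at the supplied location.
; Each asset is validity-checked, and the graph contains no movement, collision or damage logic.
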(event EventBeginPlay
  (Utilities|FlowControl|Sequence
    (:then_0
      (bind _生成音效 (Variables|Default|Get生成音效)
        (:then
          (Audio|PlaySoundatLocation _生成音效 (Transformation|GetActorLocation) "0, 0, 0" 1.0 1.0 0.0 0 0 0 0))
        (:else)))
    (:then_1
      (bind _飞行音效 (Variables|Default|Get飞行音效)
        (:then
          (Audio|SpawnSoundAttached _飞行音效 (Variables|Transformation|GetRootComponent) "None" "0, 0, 0" "0, 0, 0" "KeepRelativeOffset" true 1.0 1.0 0.0 0 0))
        (:else)))
    (:then_2
      (bind _生成时特效 (Variables|Default|Get生成时特效)
        (:then
          (Niagara|SpawnSystematLocation _生成时特效 (Transformation|GetActorLocation) (Math|Conversions|RotationFromXVector (Transformation|GetActorForwardVector))))
        (:else)))))

(event Collision|EventActorBeginOverlap
  (params (OtherActor :type Actor%20Object%20Reference)))

(event EventTick
  (params (DeltaSeconds :type Float%20%28single-precision%29)))

(event EventOnSpawnProjectileHitFx
  (params (HitLocation :type Vector%20%28by%20ref%29 :default "0, 0, 0"))
  (Utilities|FlowControl|Sequence
    (:then_0
      (bind _打击音效 (Variables|Default|Get打击音效)
        (:then
          (Audio|PlaySoundatLocation _打击音效 HitLocation "0, 0, 0" 1.0 1.0 0.0 0 0 0 0))
        (:else)))
    (:then_1
      (bind _system_template (Variables|Default|GetSystem%20Template)
        (:then
          (Niagara|SpawnSystematLocation _system_template HitLocation))
        (:else)))))

(fn ConstructionScript)