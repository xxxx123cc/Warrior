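; Base enemy Blueprint handling the dissolve-based entrance and death exit of enemy characters.
; BeginPlay plays a random montage and reverses a duration-scaled timeline driving DissolveAmount on mesh and weapon.
; The death event freezes animation, disables capsule collision, and async-loads a Niagara effect tinted by the dissolve edge color.
; The death dissolve triggers the SpawnStones ability once after a delay, then destroys weapon and enemy on finish.
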(event EventBeginPlay
  (bind _montage_to_play (Variables|Default|GetMontage%20to%20Play))
  (bind _enemycombatcomponent (Variables|Default|GetEnemyCombatComponent))
  (bind _returnvalue (Class|PawnCombatComponent|GetCurrentEquippedWeapon _enemycombatcomponent))
  (Utilities|FlowControl|Sequence
    (:then_0
      (if (Utilities|Array|IsNotEmpty _montage_to_play)
        (Animation|Montage|PlayMontage (Variables|Character|GetMesh) (.OutItem (Utilities|Array|Random _montage_to_play)))))
    (:then_1
      (Components|Timeline|SetPlayRate (Variables|Default|Get时间轴) (/ 1.0 (Variables|Default|Get入场时间)))
      (bind _新建轨道_0 (Timeline|时间轴 ReverseFromEnd)
        (:Update
          (Utilities|IsValid _returnvalue
            (:Is%20Valid
              (Rendering|Material|SetScalarParameterValueonMaterials (Variables|/Script/Warrior.WarriorWeaponBase|GetWeaponMesh _returnvalue) "DissolveAmount" _新建轨道_0))
            (:Is%20Not%20Valid
              _))
          (Rendering|Material|SetScalarParameterValueonMaterials (Variables|Character|GetMesh) "DissolveAmount" _新建轨道_0))))))

(event Collision|EventActorBeginOverlap
  (params (OtherActor :type Actor%20Object%20Reference)))

(event EventTick
  (params (DeltaSeconds :type Float%20%28single-precision%29)))

(event Event死亡退场
  (params (NewParam :type Niagara%20System%20Soft%20Object%20Reference))
  (bind _enemycombatcomponent (Variables|Default|GetEnemyCombatComponent))
  (bind _enemycombatcomponent_2 (Variables|Default|GetEnemyCombatComponent))
  (bind _mesh (Variables|Character|GetMesh))
  (bind _returnvalue (Class|PawnCombatComponent|GetCurrentEquippedWeapon _enemycombatcomponent))
  (bind _returnvalue_2 (Class|PawnCombatComponent|GetCurrentEquippedWeapon _enemycombatcomponent_2))
  (Utilities|FlowControl|Sequence
    (:then_0
      (Variables|/Script/Engine.SkeletalMeshComponent|SetbPauseAnims (Variables|Character|GetMesh) true)
      (Collision|SetCollisionEnabled (Variables|Default|GetCapsuleComponent) "NoCollision"))
    (:then_1
      (bind _object (Utilities|AsyncLoadAsset NewParam)
        (:Completed
          (bind _asniagara系统 (Utilities|Casting|CastToNiagaraSystem _object))
          (bind _returnvalue_3 (Niagara|SpawnSystemAttached _asniagara系统 (Variables|Character|GetMesh) "None" "0, 0, 0" "0, 0, 0" "KeepRelativeOffset" true))
          (bind _returnvalue_4 (Rendering|Material|CreateDynamicMaterialInstance _mesh 0 (Rendering|Material|GetMaterial _mesh 0) "None" :!class /Script/Engine.PrimitiveComponent))
          (bind _returnvalue_5 (Rendering|Material|GetVectorParameterValue _returnvalue_4 "DissolveEdgeColor" :!class /Script/Engine.MaterialInstanceDynamic))
          (Niagara|SetNiagaraVariable(LinearColor) _returnvalue_3 "DissolveParticleColor" _returnvalue_5)
          (bind _新建轨道_0 (Timeline|消失效果 PlayFromStart)
            (:Update
              (Utilities|IsValid _returnvalue
                (:Is%20Valid
                  (Rendering|Material|SetScalarParameterValueonMaterials (Variables|/Script/Warrior.WarriorWeaponBase|GetWeaponMesh _returnvalue) "DissolveAmount" _新建轨道_0))
                (:Is%20Not%20Valid
                  _))
              (Rendering|Material|SetScalarParameterValueonMaterials (Variables|Character|GetMesh) "DissolveAmount" _新建轨道_0)
              (Utilities|FlowControl|DoOnce false
                (:Completed
                  (Utilities|FlowControl|Delay 0.5)
                  (Class|WarriorAbilitySystemComponent|TryActivateAbilitybyTag (Variables|Default|GetWarriorAbilitySystemComponent) "(TagName=\"Enemy.Ability.SpawnStones\")"))))
            (:Finished
              (Utilities|IsValid _returnvalue_2
                (:Is%20Valid
                  (Actor|DestroyActor _returnvalue_2))
                (:Is%20Not%20Valid
                  _))
              (Actor|DestroyActor))))))))

(fn ConstructionScript)